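; Checkpoint hoop for a plane game that saves the respawn point and counts toward the finish line.
; On BeginPlay it turns the hoop yellow and sets FinishLine_BP's CheckPointLeft to the total number of checkpoints in the level.
; When PlanePawn_BP overlaps the trigger, it stores the plane's transform as GameMode_BP's SpawnTransform and turns the hoop lime.
; A BeenUsed flag limits the CheckPointLeft decrement to the first pass.
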(event `self.Trigger.OnComponentBeginOverlap`
  (params (OverlappedComponent :type "PrimitiveComponent Object Reference") (OtherActor :type "Actor Object Reference") (OtherComp :type "PrimitiveComponent Object Reference") (OtherBodyIndex :type Integer) (bFromSweep :type Boolean) (SweepResult :type "HitResult Structure (by ref)"))
  (bind _asplane_pawn_bp (cast `/Game/BluePrints/PlanePawn_BP` OtherActor))
  (bind _asgame_mode_bp (cast `/Game/BluePrints/GameMode_BP` (`GameplayStatics.GetGameMode`)))
  (set `/Game/BluePrints/GameMode_BP.SpawnTransform` (`self.GetTransform` _asplane_pawn_bp) _asgame_mode_bp)
  (`PrimitiveComponent.SetMaterial` (`self.Hoop`) 0 "/Game/Textures/GLTXTEST/CP_Lime_M.CP_Lime_M")
  (if (not (`self.BeenUsed`))
    (set `self.BeenUsed` true)
    (set `/Game/BluePrints/FinishLine_BP.CheckPointLeft` (- (`/Game/BluePrints/FinishLine_BP.CheckPointLeft` (stale `self.ReceiveBeginPlay` _returnvalue)) 1) (stale `self.ReceiveBeginPlay` _returnvalue))))

(event `self.ReceiveBeginPlay`
  (`PrimitiveComponent.SetMaterial` (`self.Hoop`) 0 "/Game/Textures/GLTXTEST/CP_Yellow_M.CP_Yellow_M")
  (bind _outactors (`GameplayStatics.GetAllActorsOfClass` "CheckPoint_BP_C"))
  (bind _returnvalue (`GameplayStatics.GetActorOfClass` "/Game/BluePrints/FinishLine_BP.FinishLine_BP_C"))
  (set `/Game/BluePrints/FinishLine_BP.CheckPointLeft` (`KismetArrayLibrary.Array_Length` _outactors) _returnvalue))

(fn `UserConstructionScript`)