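; Start and finish line actor that doubles as a checkpoint for the player's plane and ends the game.
; On BeginPlay it sets the game mode's SpawnTransform to its own location.
; Each PlanePawn_BP overlap with FinTrigger updates that transform to the plane's and prints a checkpoint message.
; The FinishedNow flag arms on one overlap, so a later one shows FinishText_W and quits after a short delay.
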(event `self.FinTrigger.OnComponentBeginOverlap`
  (params (OverlappedComponent :type "PrimitiveComponent Object Reference") (OtherActor :type "Actor Object Reference") (OtherComp :type "PrimitiveComponent Object Reference") (OtherBodyIndex :type Integer) (bFromSweep :type Boolean) (SweepResult :type "HitResult Structure (by ref)"))
  (bind _asplane_pawn_bp (cast `/Game/BluePrints/PlanePawn_BP` OtherActor))
  (bind _asgame_mode_bp (cast `/Game/BluePrints/GameMode_BP` (`GameplayStatics.GetGameMode`)))
  (set `/Game/BluePrints/GameMode_BP.SpawnTransform` (`self.GetTransform` _asplane_pawn_bp) _asgame_mode_bp)
  (`KismetSystemLibrary.PrintString` "CHECKPOINT")
  (if (`self.FinishedNow`)
    (bind _returnvalue (`|CreateWidget` "/Game/Widgets/FinishText_W.FinishText_W_C"))
    (bind _output_get (set `self.FinishTestVar` _returnvalue))
    (`UserWidget.AddToViewport` _output_get 0)
    (`KismetSystemLibrary.Delay` 4.0)
    (`KismetSystemLibrary.QuitGame` null "Quit")
    (else
      (set `self.FinishedNow` true))))

(event `self.ReceiveBeginPlay`
  (bind _asgame_mode_bp (cast `/Game/BluePrints/GameMode_BP` (`GameplayStatics.GetGameMode`)))
  (set `/Game/BluePrints/GameMode_BP.SpawnTransform` (`KismetMathLibrary.Conv_VectorToTransform` (`self.K2_GetActorLocation`)) _asgame_mode_bp))

(fn `UserConstructionScript`)