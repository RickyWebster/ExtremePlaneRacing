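; PosePlane is a plane Blueprint that animates its PlanePose0 mesh procedurally by setting component-space bone rotations.
; On BeginPlay it poses the two flap bones at fixed, opposing deflections and starts a fast looping timer.
; Each timer tick calls LoopAnimation, which spins the Prop bone by composing its current rotation with a small pitch increment as quaternions, turning it about its local axis.
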(event `self.ReceiveBeginPlay`
  (`KismetSystemLibrary.K2_SetTimer` null "LoopAnimation" 0.01 true)
  (bind _output_get (set `self.ElevatorAnimation` (struct :`Pitch` 1.3 :`Roll` -40.0)))
  (`PoseableMeshComponent.SetBoneRotationByName` (`self.PlanePose_0`) "Flap#1" _output_get "ComponentSpace")
  (bind _output_get_2 (set `self.ElevatorAnimation` (struct :`Pitch` -0.67 :`Yaw` 8.1 :`Roll` 40.0)))
  (`PoseableMeshComponent.SetBoneRotationByName` (`self.PlanePose_0`) "Flap#2" _output_get_2 "ComponentSpace"))

(fn `LoopAnimation`
  (bind _returnvalue (`PoseableMeshComponent.GetBoneRotationByName` (`self.PlanePose_0`) "Prop" "ComponentSpace"))
  (`PoseableMeshComponent.SetBoneRotationByName` (`self.PlanePose_0`) "Prop" (`KismetMathLibrary.Quat_Rotator` (* (`KismetMathLibrary.Conv_RotatorToQuaternion` _returnvalue) (`KismetMathLibrary.Conv_RotatorToQuaternion` (`KismetMathLibrary.MakeRotator` 0.0 1.0)))) "ComponentSpace"))

(fn `UserConstructionScript`)