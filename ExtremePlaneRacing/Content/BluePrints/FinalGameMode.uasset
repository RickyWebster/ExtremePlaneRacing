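; Game mode that respawns the player's PlanePawn_BP whenever the current pawn is destroyed.
; On BeginPlay it binds to the player pawn's OnDestroyed, then on destruction spawns a new plane at a stored transform and possesses it.
; Each respawn rebinds the event to the new pawn and holds a SpamDect flag true for a half-second delay; nothing in this graph reads the flag.
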(event `Respawn`
  (set `self.SpamDect` true)
  (bind _aspawn (cast `Pawn` (`GameplayStatics.GetPlayerPawn` 0) :!label _label))
  (add `self.OnDestroyed` _aspawn (delegate `OnRespawn`)))

(event `self.ReceiveBeginPlay`
  (goto _label))

(event `OnRespawn` :!signature `self.OnDestroyed`
  (params (DestroyedActor :type "Actor Object Reference"))
  (bind _returnvalue (`|SpawnActorFromClass` "/Game/BluePrints/PlanePawn_BP.PlanePawn_BP_C" (`self.SpawnTransform`) "Undefined" "MultiplyWithRoot" null null))
  (`Controller.Possess` (`GameplayStatics.GetPlayerController` 0) _returnvalue)
  (`self.Respawn`)
  (`KismetSystemLibrary.Delay` 0.5)
  (set `self.SpamDect` false))

(fn `UserConstructionScript`)